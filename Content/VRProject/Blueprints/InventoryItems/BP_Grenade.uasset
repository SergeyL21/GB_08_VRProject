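; BP_Grenade is a VR inventory item that simulates a timed grenade using debug text only.
; The first trigger release starts a looping one-second timer, with a DoOnce ignoring later releases.
; Each tick passes through a DoN counter that prints numbered "PIP" messages, then "*BOOM*" on the fifth and final count.
; No damage, effects or timer clearing are implemented here.
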(event Custom|GrenadeTimer
  (bind _counter (Utilities|FlowControl|DoN 5)
    (:Exit
      (if (== _counter 5)
        (Development|PrintString "*BOOM*" true true "(R=1.000000,G=0.053064,B=0.000000,A=1.000000)" 1.0)
        (else
          (Development|PrintString (Utilities|String|ToString(Text) (Utilities|Text|FormatText "*PIP {0}*" (Utilities|Text|ToText(Integer) _counter))) true true "(R=0.000000,G=0.660000,B=1.000000,A=1.000000)" 1.0))))))

(event EventTriggerReleased
  (Utilities|FlowControl|DoOnce false
    (:Completed
      (Utilities|Time|SetTimerbyEvent (delegate Custom|GrenadeTimer) 1.0 true))))

(fn ConstructionScript
  (|CallParentFunction))