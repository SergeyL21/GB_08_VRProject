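; BP_Weapon is a hitscan weapon in the VR project's inventory items, fired on the TriggerPressed event.
; It line-traces along the muzzle's forward vector on the Visibility channel, drawing a one-frame debug line.
; A hit applies fixed damage, spawns BP_Explosion at the hit location and adds an impulse to the hit component.
; That impulse is scaled from the world-space impact point, not the shot direction.
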(event EventTriggerPressed
  (bind _muzzlelocation (Variables|Default|GetMuzzleLocation))
  (bind _returnvalue (Transformation|GetWorldLocation _muzzlelocation))
  (bind (_outhit _returnvalue_2) (Collision|LineTraceByChannel _returnvalue (+ _returnvalue (* (Math|Vector|GetForwardVector _muzzlelocation) 99999.0)) "TraceTypeQuery1" true 0 "ForOneFrame"))
  (if _returnvalue_2
    (Game|Damage|ApplyDamage (.HitActor (Collision|BreakHitResult _outhit)) 1e+02 0 0)
    (Physics|AddImpulse (.HitComponent (Collision|BreakHitResult _outhit)) (* (.ImpactPoint (Collision|BreakHitResult _outhit)) 1e+02) "None" false)
    (Game|SpawnActorfromClass "/Game/VRProject/Blueprints/BP_Explosion.BP_Explosion_C" (Math|Conversions|ToTransform(Vector) (.Location (Collision|BreakHitResult _outhit))) "AlwaysSpawn" (.HitActor (Collision|BreakHitResult _outhit)) 0)))

(fn ConstructionScript)