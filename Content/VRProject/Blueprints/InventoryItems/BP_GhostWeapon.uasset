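; BP_GhostWeapon is a VR project weapon that shoots through destructible objects to hit the last one in line.
; Trigger press runs a long multi-object line trace forward from the muzzle, filtered to Destructible objects.
; Only the final hit takes damage and receives an impulse, derived from its world impact point rather than shot direction.
; Every hit's index and name prints on screen as debug output.
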(event EventTriggerPressed
  (bind _muzzlelocation (Variables|Default|GetMuzzleLocation))
  (bind _returnvalue (Transformation|GetWorldLocation _muzzlelocation))
  (bind _outhits (Class|KismetSystemLibrary|LineTraceMultiforObjects _returnvalue (+ _returnvalue (* (Math|Vector|GetForwardVector _muzzlelocation) 99999.0)) (Utilities|Array|MakeArray "ObjectTypeQuery6") false 0 "ForOneFrame" true))
  (for (_array_element _array_index) _outhits
    (if (== _array_index (Utilities|Array|LastIndex _outhits))
      (Game|Damage|ApplyDamage (.HitActor (Collision|BreakHitResult _array_element)) 1e+02 0 0)
      (Physics|AddImpulse (.HitComponent (Collision|BreakHitResult _array_element)) (* (.ImpactPoint (Collision|BreakHitResult _array_element)) 1e+01) "None" false))
    (Development|PrintString (Utilities|String|ToString(Text) (Utilities|Text|FormatText "ARRAY N={Index} Name={Name}" _array_index (Utilities|GetDisplayName (.HitActor (Collision|BreakHitResult _array_element))))) true true "(R=1.000000,G=0.007140,B=0.000000,A=1.000000)" 1e+01)))

(fn ConstructionScript)