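; BP_InventorySlot is an inventory slot for the VR project that tracks which BP_InventoryItem is inside it.
; Its static mesh's begin overlap stores the overlapping item as ItemInSlot, and end overlap clears it if that same item leaves.
; The Put event calls TryGrab on the stored item's GrabComponent with a MotionController, without checking that the slot is occupied.
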(event OnComponentBeginOverlap(StaticMesh)
  (params (OverlappedComponent :type Primitive%20Component%20Object%20Reference) (OtherActor :type Actor%20Object%20Reference) (OtherComp :type Primitive%20Component%20Object%20Reference) (OtherBodyIndex :type Integer) (bFromSweep :type Boolean) (SweepResult :type Hit%20Result%20Structure%20%28by%20ref%29))
  (bind _asbp_inventory_item (Utilities|Casting|CastToBP_InventoryItem OtherActor))
  (Variables|Default|SetItemInSlot _asbp_inventory_item))

(event OnComponentEndOverlap(StaticMesh)
  (params (OverlappedComponent :type Primitive%20Component%20Object%20Reference) (OtherActor :type Actor%20Object%20Reference) (OtherComp :type Primitive%20Component%20Object%20Reference) (OtherBodyIndex :type Integer))
  (bind _asbp_inventory_item (Utilities|Casting|CastToBP_InventoryItem OtherActor))
  (if (== _asbp_inventory_item (Variables|Default|GetItemInSlot))
    (Variables|Default|SetItemInSlot 0)))

(event Custom|Put
  (Default|TryGrab (Variables|/Game/VRProject/Blueprints/BP_Interaction.BP_Interaction_C|GetGrabComponent (Variables|Default|GetItemInSlot)) (Variables|Default|GetMotionController)))

(fn ConstructionScript)