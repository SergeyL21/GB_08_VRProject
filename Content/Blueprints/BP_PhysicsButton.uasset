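; BP_PhysicsButton is a button that reacts when its Cylinder is displaced from its starting position.
; Tick measures the distance from the location cached at BeginPlay, showing a green material past a small threshold and red otherwise.
; A DoOnce sends an Interact message to PointLight once per press, resetting when the Cylinder returns within range.
; Its own Interact event toggles PointLight visibility.
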(event EventBeginPlay
  (Variables|Default|SetButtonStartLocation (Transformation|GetWorldLocation (Variables|Default|GetCylinder))))

(event EventTick
  (params (DeltaSeconds :type Float%20%28single-precision%29))
  (bind _cylinder (Variables|Default|GetCylinder))
  (if (> (Math|Vector|VectorLength (- (Variables|Default|GetButtonStartLocation) (Transformation|GetWorldLocation (Variables|Default|GetCylinder)))) 4.0)
    (Rendering|Material|SetMaterial _cylinder 0 "/Game/Materials/MI_GreenMaterial.MI_GreenMaterial")
    (Utilities|FlowControl|DoOnce false :!label _label
      (:Completed
        (Class|BPIVRInteract|Interact(Message) (Variables|Default|GetPointLight))))
    (else
      (Rendering|Material|SetMaterial _cylinder 0 "/Game/Materials/MI_RedMaterial.MI_RedMaterial")
      (goto _label Reset))))

(event EventInteract
  (Rendering|ToggleVisibility (Variables|Default|GetPointLight) false))

(fn ConstructionScript)