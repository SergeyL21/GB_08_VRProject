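; VR push button that sends an Interact message to PointLight when a BP_VRCharacter presses it.
; Overlap begin and end play and reverse a Timeline that drives the Cylinder's Z location.
; Below a height threshold the cylinder turns green and a DoOnce fires the message; above it, the cylinder turns red and re-arms.
; Its own Interact event toggles PointLight visibility.
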(event OnComponentBeginOverlap(Cylinder)
  (params (OverlappedComponent :type Primitive%20Component%20Object%20Reference) (OtherActor :type Actor%20Object%20Reference) (OtherComp :type Primitive%20Component%20Object%20Reference) (OtherBodyIndex :type Integer) (bFromSweep :type Boolean) (SweepResult :type Hit%20Result%20Structure%20%28by%20ref%29))
  (bind _cylinder (Variables|Default|GetCylinder))
  (Utilities|Casting|CastToBP_VRCharacter OtherActor)
  (bind _buttonz (Timeline|Timeline Play)
    (:Update
      (Transformation|SetRelativeLocation (Variables|Default|GetCylinder) (Math|Vector|MakeVector 0.0 0.0 _buttonz) false false)
      (if (< _buttonz 46.0)
        (Rendering|Material|SetMaterial _cylinder 0 "/Game/Materials/MI_GreenMaterial.MI_GreenMaterial")
        (Utilities|FlowControl|DoOnce false :!label _label
          (:Completed
            (Class|BPIVRInteract|Interact(Message) (Variables|Default|GetPointLight))))
        (else
          (Rendering|Material|SetMaterial _cylinder 0 "/Game/Materials/MI_RedMaterial.MI_RedMaterial")
          (goto _label Reset))))))

(event OnComponentEndOverlap(Cylinder)
  (params (OverlappedComponent :type Primitive%20Component%20Object%20Reference) (OtherActor :type Actor%20Object%20Reference) (OtherComp :type Primitive%20Component%20Object%20Reference) (OtherBodyIndex :type Integer))
  (bind _cylinder (Variables|Default|GetCylinder))
  (Utilities|Casting|CastToBP_VRCharacter OtherActor)
  (bind _buttonz (Timeline|Timeline Reverse)
    (:Update
      (Transformation|SetRelativeLocation (Variables|Default|GetCylinder) (Math|Vector|MakeVector 0.0 0.0 _buttonz) false false)
      (if (< _buttonz 46.0)
        (Rendering|Material|SetMaterial _cylinder 0 "/Game/Materials/MI_GreenMaterial.MI_GreenMaterial")
        (Utilities|FlowControl|DoOnce false :!label _label
          (:Completed
            (Class|BPIVRInteract|Interact(Message) (Variables|Default|GetPointLight))))
        (else
          (Rendering|Material|SetMaterial _cylinder 0 "/Game/Materials/MI_RedMaterial.MI_RedMaterial")
          (goto _label Reset))))))

(event EventInteract
  (Rendering|ToggleVisibility (Variables|Default|GetPointLight) false))

(fn ConstructionScript)