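; VR player character with camera-relative movement, teleporting and two-handed grabbing; its body mesh follows the headset's horizontal position and yaw each tick.
; Teleport runs a timer-driven projectile arc from the right controller, projects the hit onto the navmesh, and moves the player on release.
; Grips message overlapped BPI_VRGrip components, adding physics constraints for those tagged "physics".
; Grip axes store hand states, and overlap events set right-hand finger flags.
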(event EventTick
  (params (DeltaSeconds :type Float%20%28single-precision%29))
  (bind (_location _rotation) (CallFunction|LocationandRotation))
  (Transformation|SetWorldLocationAndRotation (Variables|Character|GetMesh) _location _rotation false false))

(event Input|ActionEvents|InputActionTeleport
  (params (Key :type Key%20Structure))
  (:Pressed
    (CallFunction|ActivateTeleport))
  (:Released
    (CallFunction|DeactivateTeleport)))

(event Input|ActionEvents|InputActionGripLeft
  (params (Key :type Key%20Structure))
  (:Pressed
    (bind _primitivecomponent (CallFunction|TryGrip (Variables|Default|GetLeftPhysicsConstraint) (Variables|Components|GetLeftGrabSphere)))
    (bind _output_get (Variables|Default|SetLeftGripPrimitiveComponent _primitivecomponent))
    (Class|BPIVRGrip|Grip(Message) _output_get (Variables|Components|GetMotionControllerLeft)))
  (:Released
    (bind _result (CallFunction|TryDrop (Variables|Default|GetLeftGripPrimitiveComponent) (Variables|Default|GetLeftPhysicsConstraint)))
    (if _result
      (Variables|Default|SetLeftGripPrimitiveComponent 0))))

(event Input|ActionEvents|InputActionGripRight
  (params (Key :type Key%20Structure))
  (:Pressed
    (bind _primitivecomponent (CallFunction|TryGrip (Variables|Default|GetRightPhysicsConstraint) (Variables|Components|GetRightGrabSphere)))
    (bind _output_get (Variables|Default|SetRightGripPrimitiveComponent _primitivecomponent))
    (Class|BPIVRGrip|Grip(Message) _output_get (Variables|Components|GetMotionControllerLeft)))
  (:Released
    (bind _result (CallFunction|TryDrop (Variables|Default|GetRightGripPrimitiveComponent) (Variables|Default|GetRightPhysicsConstraint)))
    (if _result
      (Variables|Default|SetRightGripPrimitiveComponent 0))))

(event Input|AxisEvents|InputAxisMoveForward
  (params (AxisValue :type Float%20%28single-precision%29))
  (Pawn|Input|AddMovementInput (Math|Vector|GetForwardVector (Math|Rotator|MakeRotator 0.0 0.0 (.yaw (Transformation|GetWorldRotation (Variables|Components|GetCamera))))) AxisValue false))

(event Input|AxisEvents|InputAxisMoveRight
  (params (AxisValue :type Float%20%28single-precision%29))
  (Pawn|Input|AddMovementInput (Math|Vector|GetRightVector (Math|Rotator|MakeRotator 0.0 0.0 (.yaw (Transformation|GetWorldRotation (Variables|Components|GetCamera))))) AxisValue false))

(event Input|AxisEvents|InputAxisGripLeftAxis
  (params (AxisValue :type Float%20%28single-precision%29))
  (Variables|Default|SetLeftGripState AxisValue))

(event Input|AxisEvents|InputAxisGripRightAxis
  (params (AxisValue :type Float%20%28single-precision%29))
  (Variables|Default|SetRightGripState AxisValue))

(event OnComponentEndOverlap(RightMiddle1)
  (params (OverlappedComponent :type Primitive%20Component%20Object%20Reference) (OtherActor :type Actor%20Object%20Reference) (OtherComp :type Primitive%20Component%20Object%20Reference) (OtherBodyIndex :type Integer))
  (Variables|RightHandCollision|SetRightMiddle false))

(event OnComponentBeginOverlap(RightRing1)
  (params (OverlappedComponent :type Primitive%20Component%20Object%20Reference) (OtherActor :type Actor%20Object%20Reference) (OtherComp :type Primitive%20Component%20Object%20Reference) (OtherBodyIndex :type Integer) (bFromSweep :type Boolean) (SweepResult :type Hit%20Result%20Structure%20%28by%20ref%29))
  (Variables|RightHandCollision|SetRightRing true))

(event OnComponentEndOverlap(RightRing1)
  (params (OverlappedComponent :type Primitive%20Component%20Object%20Reference) (OtherActor :type Actor%20Object%20Reference) (OtherComp :type Primitive%20Component%20Object%20Reference) (OtherBodyIndex :type Integer))
  (Variables|RightHandCollision|SetRightRing false))

(event OnComponentBeginOverlap(RightThumb1)
  (params (OverlappedComponent :type Primitive%20Component%20Object%20Reference) (OtherActor :type Actor%20Object%20Reference) (OtherComp :type Primitive%20Component%20Object%20Reference) (OtherBodyIndex :type Integer) (bFromSweep :type Boolean) (SweepResult :type Hit%20Result%20Structure%20%28by%20ref%29))
  (Variables|RightHandCollision|SetRightThumb true))

(event OnComponentEndOverlap(RightGrabSphere)
  (params (OverlappedComponent :type Primitive%20Component%20Object%20Reference) (OtherActor :type Actor%20Object%20Reference) (OtherComp :type Primitive%20Component%20Object%20Reference) (OtherBodyIndex :type Integer))
  (Variables|RightHandCollision|SetRightThumb false))

(event OnComponentBeginOverlap(RightIndex1)
  (params (OverlappedComponent :type Primitive%20Component%20Object%20Reference) (OtherActor :type Actor%20Object%20Reference) (OtherComp :type Primitive%20Component%20Object%20Reference) (OtherBodyIndex :type Integer) (bFromSweep :type Boolean) (SweepResult :type Hit%20Result%20Structure%20%28by%20ref%29))
  (Variables|RightHandCollision|SetRightIndex true))

(event OnComponentEndOverlap(RightIndex1)
  (params (OverlappedComponent :type Primitive%20Component%20Object%20Reference) (OtherActor :type Actor%20Object%20Reference) (OtherComp :type Primitive%20Component%20Object%20Reference) (OtherBodyIndex :type Integer))
  (Variables|RightHandCollision|SetRightIndex false))

(event OnComponentBeginOverlap(RightMiddle1)
  (params (OverlappedComponent :type Primitive%20Component%20Object%20Reference) (OtherActor :type Actor%20Object%20Reference) (OtherComp :type Primitive%20Component%20Object%20Reference) (OtherBodyIndex :type Integer) (bFromSweep :type Boolean) (SweepResult :type Hit%20Result%20Structure%20%28by%20ref%29))
  (Variables|RightHandCollision|SetRightMiddle true))

(fn ConstructionScript)

(fn ActivateTeleport
  (if (not (Variables|Default|GetIsTeleportActivated))
    (Variables|Default|SetIsTeleportActivated true)
    (Rendering|SetVisibility (Variables|Components|GetTeleportMesh) true false)
    (bind _returnvalue (Utilities|Time|SetTimerbyFunctionName 0 "UpdateTraceTeleport" 0.1 true))
    (Variables|Default|SetTeleportTimerHandle _returnvalue)))

(fn UpdateTraceTeleport
  (bind _motioncontrollerright (Variables|Components|GetMotionControllerRight))
  (bind _teleportmesh (Variables|Components|GetTeleportMesh))
  (bind _returnvalue (Math|Vector|GetForwardVector _motioncontrollerright))
  (bind _outhit (Class|GameplayStatics|BlueprintPredictProjectilePathbyTraceChannel (+ (Transformation|GetWorldLocation _motioncontrollerright) (* _returnvalue 1e+02)) (* _returnvalue (Variables|Default|GetTeleportVelocity)) true 3e+01 "ECC_WorldStatic" false 0 "ForDuration"))
  (Transformation|SetWorldLocation _teleportmesh (.ProjectedLocation (AI|Navigation|ProjectPointtoNavigation (Class|NavigationSystemV1|GetNavigationSystem) (.Location (Collision|BreakHitResult _outhit)) 0 0 "200.000000,200.000000,100.000000")) false false)
  (Rendering|SetVisibility _teleportmesh (.ReturnValue (AI|Navigation|ProjectPointtoNavigation (Class|NavigationSystemV1|GetNavigationSystem) (.Location (Collision|BreakHitResult _outhit)) 0 0 "200.000000,200.000000,100.000000")) false)
  (Variables|Default|SetCanTeleport (.ReturnValue (AI|Navigation|ProjectPointtoNavigation (Class|NavigationSystemV1|GetNavigationSystem) (.Location (Collision|BreakHitResult _outhit)) 0 0 "200.000000,200.000000,100.000000"))))

(fn DeactivateTeleport
  (bind _teleportmesh (Variables|Components|GetTeleportMesh))
  (if (Utilities|Time|IsValidTimerHandle (Variables|Default|GetTeleportTimerHandle))
    (Utilities|Time|ClearandInvalidateTimerbyHandle (Variables|Default|GetTeleportTimerHandle))
    (Variables|Default|SetTeleportTimerHandle "")
    (Variables|Default|SetIsTeleportActivated false)
    (Rendering|SetVisibility (Variables|Components|GetTeleportMesh) false false)
    (if (Variables|Default|GetCanTeleport)
      (Transformation|SetActorLocation (+ (Transformation|GetWorldLocation _teleportmesh) "0, 0,90.000000") false false)
      (Transformation|SetWorldRotation (Variables|Components|GetVROrigin) (Transformation|GetWorldRotation _teleportmesh) false false))))

(fn LocationandRotation
  (bind _mesh (Variables|Character|GetMesh))
  (bind _camera (Variables|Components|GetCamera))
  (bind _returnvalue (Transformation|GetWorldTransform _camera))
  (bind _returnvalue_2 (Transformation|GetWorldTransform _mesh))
  (bind (_roll _pitch) (Math|Rotator|BreakRotator (.rotation _returnvalue_2)))
  (bind (_x _y) (Math|Vector|BreakVector (.location _returnvalue)))
  (return (Math|Vector|MakeVector _x _y (.Z (Math|Vector|BreakVector (.location _returnvalue_2)))) (Math|Rotator|MakeRotator _roll _pitch (.Yaw (Math|Rotator|BreakRotator (.rotation _returnvalue))))))

(fn TryGrip
  (params (PhysicsConstraint :type Physics%20Constraint%20Component%20Object%20Reference) (GrabCollision :type Primitive%20Component%20Object%20Reference))
  (bind _outoverlappingcomponents (Class|PrimitiveComponent|GetOverlappingComponents GrabCollision))
  (bind _returnvalue (Utilities|Array|LastIndex _outoverlappingcomponents))
  (bind _output (Utilities|Array|Get(acopy) _outoverlappingcomponents _returnvalue))
  (if (Utilities|DoesObjectImplementInterface _output "/Game/Blueprints/BPI_VRGrip.BPI_VRGrip_C")
    (if (Components|ComponentHasTag _output "physics")
      (Class|PhysicsConstraintComponent|SetConstrainedComponents PhysicsConstraint GrabCollision "None" _output "None")
      (Collision|SetCollisionResponsetoChannel _output "ECC_Pawn" "ECR_Ignore"))
    (return _output)))

(fn TryDrop
  (params (GripPrimitiveComponent :type Primitive%20Component%20Object%20Reference) (PhysicsConstraint :type Physics%20Constraint%20Component%20Object%20Reference))
  (Utilities|IsValid GripPrimitiveComponent
    (:Is%20Valid
      (Class|BPIVRGrip|Drop(Message) GripPrimitiveComponent)
      (return true))
    (:Is%20Not%20Valid
      (Class|PhysicsConstraintComponent|BreakConstraint PhysicsConstraint)
      (Collision|SetCollisionResponsetoChannel GripPrimitiveComponent "ECC_Pawn" "ECR_Block")
      (return false))))