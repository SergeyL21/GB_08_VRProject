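; BP_CustomGrapActor is a lesson actor that the player can grab and drop, driven by a grip component.
; On BeginPlay it binds handlers to the component's grip and drop events.
; Gripping turns off physics simulation and attaches the component to the interacting component, keeping world location and rotation.
; Dropping re-enables physics and detaches it.
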(event Custom|OnDropped
  (bind _bpc_gripcomponent (Variables|Default|GetBPC_GripComponent))
  (Physics|SetSimulatePhysics _bpc_gripcomponent true)
  (Transformation|DetachFromComponent _bpc_gripcomponent "KeepRelative" "KeepRelative" "KeepRelative" true))

(event Custom|OnGripped
  (params (Interaction :type Motion%20Controller%20Component%20Object%20Reference))
  (bind _bpc_gripcomponent (Variables|Default|GetBPC_GripComponent))
  (Physics|SetSimulatePhysics _bpc_gripcomponent false)
  (Transformation|AttachComponentToComponent _bpc_gripcomponent Interaction "None" "KeepWorld" "KeepWorld" "KeepRelative" true))

(event EventBeginPlay
  (EventDispatchers|BindEventtoOnDrop (Variables|Default|GetBPC_GripComponent) (EventDispatchers|CreateEvent :!event Custom|OnDropped))
  (EventDispatchers|BindEventtoOnGrip (Variables|Default|GetBPC_GripComponent) (EventDispatchers|CreateEvent :!event Custom|OnGripped)))

(fn ConstructionScript)