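; BP_Panel is a display panel that runs a timed, data-table-driven button-matching level and shows prompts and score.
; It binds to every BP_GameButton in the world, showing "UNDER CONSTRUCTION" if none exist, and routes presses through a Start, In Progress, Finish state.
; After a delayed "PREPARE", each row's comma-separated signs are cleared by matching presses in any order.
; A looping timer tracks time so faster rows score more, until rows run out.
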(event Custom|OnGameButtonPressed
  (params (Sign :type Text))
  (bind _textelement (Variables|Default|GetTextElement))
  (switch Utilities|FlowControl|Switch|SwitchonE_LevelState (Variables|Default|GetLevelState)
    (:NewEnumerator0
      (CallFunction|StartLevelSequence))
    (:NewEnumerator1
      (CallFunction|UpdateCurrentSequence Sign))
    (:NewEnumerator2
      (Rendering|Components|TextRender|SetWorldSize _textelement 52.0)
      (Rendering|Components|TextRender|SetText _textelement (Utilities|Text|FormatText "LEVEL COMPLETED 
PRESS KEY \"Trigger 
Right\" TO GO TO 
NEXT LEVEL")))))

(event EventBeginPlay
  (bind _textelement (Variables|Default|GetTextElement))
  (Rendering|Components|TextRender|SetText (Variables|Default|GetTextElement) (Utilities|Text|FormatText "PRESS ANY 
BUTTON TO 
START"))
  (bind _outactors (Actor|GetAllActorsOfClass "/Game/Blueprints/Game/BP_GameButton.BP_GameButton_C"))
  (for _array_element _outactors
    (bind _asbp_game_button (Utilities|Casting|CastToBP_GameButton _array_element))
    (EventDispatchers|AssignGameButtonPressed _asbp_game_button (delegate Custom|OnGameButtonPressed)))
  (if (== (Utilities|Array|Length _outactors) 0)
    (Rendering|Components|TextRender|SetTextRenderColor _textelement (Math|Color|MakeColor 0 0 255 255))
    (Rendering|Components|TextRender|SetWorldSize _textelement 64.0)
    (Rendering|Components|TextRender|SetText _textelement (Utilities|Text|FormatText "UNDER 
CONSTRUCTION"))))

(fn ConstructionScript)

(fn StartLevelSequence
  (if (not (Utilities|Time|IsValidTimerHandle (Variables|Default|GetLevelTimerHandle)))
    _
    (else
      (Utilities|Time|ClearandInvalidateTimerbyHandle (Variables|Default|GetLevelTimerHandle))))
  (Variables|Default|SetLevelState "NewEnumerator0")
  (Variables|Default|SetCurrentLevelTime 0.0)
  (Variables|Default|SetPlayerScore 0)
  (Variables|Default|SetCurrentTableRowIndex 0)
  (Utilities|Array|Clear (Variables|Default|GetCurrentRowSigns))
  (Variables|Default|SetCurrentTableRow "")
  (CallFunction|NextTableRowbyIndex (Variables|Default|GetCurrentTableRowIndex))
  (bind _returnvalue (Utilities|Time|SetTimerbyFunctionName self "OnLevelSequenceStarted" 3.0))
  (Variables|Default|SetLevelTimerHandle _returnvalue)
  (Rendering|Components|TextRender|SetText (Variables|Default|GetTextElement) (Utilities|Text|FormatText "PREPARE"))
  (return))

(fn NextLevelSequence
  (Utilities|Time|PauseTimerbyHandle (Variables|Default|GetLevelTimerHandle))
  (Variables|Default|SetPlayerScore (+ (Math|Float|Truncate (* (/ 2.0 (Variables|Default|GetCurrentLevelTime)) 1e+02)) (Variables|Default|GetPlayerScore)))
  (Variables|Default|SetCurrentLevelTime 0.0)
  (bind _result (Math|Integer|IncrementInt (Variables|Default|GetCurrentTableRowIndex))
    (:%20%20
      (bind _result_2 (CallFunction|NextTableRowbyIndex _result))
      (if _result_2
        (CallFunction|UpdatePanelText)
        (Utilities|Time|UnpauseTimerbyHandle (Variables|Default|GetLevelTimerHandle))
        (else
          (Variables|Default|SetLevelState "NewEnumerator2"))))))

(fn NextTableRowbyIndex
  (params (Index :type Integer))
  (bind _outrownames (DataTable|GetDataTableRowNames (Variables|Default|GetLevelTable)))
  (if (Utilities|Array|IsValidIndex _outrownames Index)
    (bind _returnvalue (Utilities|GetDataTableRow (Variables|Default|GetLevelTable) (Utilities|Array|Get(acopy) _outrownames Index))
      (:then
        (Variables|Default|SetCurrentTableRow (Utilities|Struct|MakeLevelDataElement (Utilities|Struct|BreakLevelDataElement _returnvalue)))
        (Variables|Default|SetCurrentRowSigns (Utilities|String|ParseIntoArray (Utilities|String|ToString(Text) (Utilities|Struct|BreakLevelDataElement _returnvalue)) ","))
        (return true))
      (:RowNotFound
        (Variables|Default|SetCurrentRowSigns (Utilities|Array|MakeArray ""))
        (return false)))))

(fn UpdateCurrentSequence
  (params (Sign :type Text))
  (bind _currentrowsigns (Variables|Default|GetCurrentRowSigns))
  (Utilities|Array|RemoveIndex _currentrowsigns (Utilities|Array|FindItem _currentrowsigns (Utilities|String|ToString(Text) Sign)))
  (if (== (Utilities|Array|Length _currentrowsigns) 0)
    (CallFunction|NextLevelSequence))
  (return))

(fn OnLevelSequenceStarted
  (bind _returnvalue (Utilities|Time|SetTimerbyFunctionName self "OnLevelTimeout" 0.1 true))
  (Utilities|Time|ClearandInvalidateTimerbyHandle (Variables|Default|GetLevelTimerHandle))
  (Variables|Default|SetLevelTimerHandle _returnvalue)
  (Variables|Default|SetLevelState "NewEnumerator1")
  (CallFunction|UpdatePanelText))

(fn UpdatePanelText
  (Rendering|Components|TextRender|SetText (Variables|Default|GetTextElement) (.signs (Variables|Default|GetCurrentTableRow)))
  (Rendering|Components|TextRender|SetText (Variables|Default|GetTextScore) (Utilities|Text|FormatText "SCORE: {Value}" (Variables|Default|GetPlayerScore))))

(fn OnLevelTimeout
  (Variables|Default|SetCurrentLevelTime (+ (Class|KismetSystemLibrary|GetTimerElapsedTimeHandle (Variables|Default|GetLevelTimerHandle)) (Variables|Default|GetCurrentLevelTime))))

(fn GetLevelState
  (return (Variables|Default|GetLevelState)))