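; Pressable game button with a text label set from ButtonText in the construction script.
; Overlapping the cylinder toggles a point light and plays a timeline that moves the cylinder's Z; ending the overlap reverses it.
; Below a height threshold the cap turns green and sends Interact once, re-armed when it rises back to red.
; The Interact event broadcasts GameButtonPressed with the button's text.
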(event OnComponentBeginOverlap(Cylinder)
  (params (OverlappedComponent :type Primitive%20Component%20Object%20Reference) (OtherActor :type Actor%20Object%20Reference) (OtherComp :type Primitive%20Component%20Object%20Reference) (OtherBodyIndex :type Integer) (bFromSweep :type Boolean) (SweepResult :type Hit%20Result%20Structure%20%28by%20ref%29))
  (bind _cylinder (Variables|Default|GetCylinder))
  (Rendering|ToggleVisibility (Variables|Default|GetPointLight) false)
  (bind _buttonz (Timeline|Timeline Play)
    (:Update
      (Transformation|SetRelativeLocation (Variables|Default|GetCylinder) (Math|Vector|MakeVector 0.0 0.0 _buttonz) false false)
      (if (< _buttonz 46.0)
        (Rendering|Material|SetMaterial _cylinder 0 "/Game/Materials/MI_GreenMaterial.MI_GreenMaterial")
        (Utilities|FlowControl|DoOnce false :!label _label
          (:Completed
            (Class|BPIVRInteract|Interact(Message) self)))
        (else
          (Rendering|Material|SetMaterial _cylinder 0 "/Game/Materials/MI_RedMaterial.MI_RedMaterial")
          (goto _label Reset))))
    (:Finished
      (Rendering|SetVisibility (Variables|Default|GetPointLight) false false))))

(event OnComponentEndOverlap(Cylinder)
  (params (OverlappedComponent :type Primitive%20Component%20Object%20Reference) (OtherActor :type Actor%20Object%20Reference) (OtherComp :type Primitive%20Component%20Object%20Reference) (OtherBodyIndex :type Integer))
  (bind _cylinder (Variables|Default|GetCylinder))
  (Rendering|ToggleVisibility (Variables|Default|GetPointLight) false)
  (bind _buttonz (Timeline|Timeline Reverse)
    (:Update
      (Transformation|SetRelativeLocation (Variables|Default|GetCylinder) (Math|Vector|MakeVector 0.0 0.0 _buttonz) false false)
      (if (< _buttonz 46.0)
        (Rendering|Material|SetMaterial _cylinder 0 "/Game/Materials/MI_GreenMaterial.MI_GreenMaterial")
        (Utilities|FlowControl|DoOnce false :!label _label
          (:Completed
            (Class|BPIVRInteract|Interact(Message) self)))
        (else
          (Rendering|Material|SetMaterial _cylinder 0 "/Game/Materials/MI_RedMaterial.MI_RedMaterial")
          (goto _label Reset))))
    (:Finished
      (Rendering|SetVisibility (Variables|Default|GetPointLight) false false))))

(event EventInteract
  (Default|CallGameButtonPressed (Variables|Default|GetButtonText)))

(fn ConstructionScript
  (Rendering|Components|TextRender|SetText (Variables|Default|GetTextRender) (Variables|Default|GetButtonText)))