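; BP_GamePawn is the player pawn that handles a world-space level menu and progression to the next level.
; The Menu input shows the widget and its interaction pointer with debug display, and the menu's close event hides both.
; The left trigger acts as a mouse click on the widget.
; The right trigger opens the next level named by the last BP_Panel found at BeginPlay, if its level state allows.
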(event Custom|OnMenuClosed
  (Development|PrintString "Hello")
  (Components|Activation|SetActive (Variables|Default|GetWidgetInteraction) false false)
  (Variables|/Script/UMG.WidgetInteractionComponent|SetbShowDebug (Variables|Default|GetWidgetInteraction) false)
  (Rendering|SetVisibility (Variables|Default|GetMenuWidget) false false))

(event EventBeginPlay
  (bind _outactors (Actor|GetAllActorsOfClass "/Game/Blueprints/Game/BP_Panel.BP_Panel_C"))
  (Variables|Default|SetGamePanel (Utilities|Array|Get(acopy) _outactors (Utilities|Array|LastIndex _outactors)))
  (bind _aswbp_level_menu (Utilities|Casting|CastToWBP_LevelMenu (UserInterface|GetWidget (Variables|Default|GetMenuWidget))))
  (EventDispatchers|BindEventtoOnButtonClosePressed _aswbp_level_menu (delegate Custom|OnMenuClosed)))

(event Input|ActionEvents|InputActionMenu
  (params (Key :type Key%20Structure :default "None"))
  (:Pressed
    (Components|Activation|SetActive (Variables|Default|GetWidgetInteraction) true false)
    (Variables|/Script/UMG.WidgetInteractionComponent|SetbShowDebug (Variables|Default|GetWidgetInteraction) true)
    (Rendering|SetVisibility (Variables|Default|GetMenuWidget) true false)))

(event Input|ActionEvents|InputActionTriggerLeft
  (params (Key :type Key%20Structure :default "None"))
  (bind _widgetinteraction (Variables|Default|GetWidgetInteraction))
  (:Pressed
    (Class|WidgetInteractionComponent|PressPointerKey _widgetinteraction "LeftMouseButton"))
  (:Released
    (Class|WidgetInteractionComponent|ReleasePointerKey _widgetinteraction "LeftMouseButton")))

(event Input|ActionEvents|InputActionTriggerRight
  (params (Key :type Key%20Structure :default "None"))
  (:Pressed
    (if (Utilities|Enum|Equal(Enum) (Default|GetLevelState (Variables|Default|GetGamePanel)) "NewEnumerator2")
      (Game|OpenLevel(byName) (Variables|/Game/Blueprints/Game/BP_Panel.BP_Panel_C|GetNextLevelName (Variables|Default|GetGamePanel))))))

(fn ConstructionScript)